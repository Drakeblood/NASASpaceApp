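; BP_Dialogue is an interactable actor that shows a dialogue message on the player's HUD.
; Focus and Unfocus show and hide its Widget component, and CanInteract always returns true.
; Interact casts the caller to BP_HeroCharacter and its controller to BP_PlayerController, then passes the actor's Text and Duration to ShowDialogue on that controller's HUD widget.
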(event EventBeginPlay)

(event Collision|EventActorBeginOverlap
  (params (OtherActor :type Actor%20Object%20Reference)))

(event EventTick
  (params (DeltaSeconds :type Float%20%28single-precision%29)))

(event EventFocus
  (params (Caller :type Actor%20Object%20Reference))
  (Rendering|SetVisibility (Variables|Default|GetWidget) true false))

(event EventUnfocus
  (params (Caller :type BP%20Hero%20Character%20Object%20Reference))
  (Rendering|SetVisibility (Variables|Default|GetWidget) false false))

(event EventInteract
  (params (Caller :type Actor%20Object%20Reference))
  (bind _asbp_hero_character (Utilities|Casting|CastToBP_HeroCharacter Caller))
  (bind _asbp_player_controller (Utilities|Casting|CastToBP_PlayerController (Pawn|GetController _asbp_hero_character)))
  (Default|ShowDialogue (Variables|/Game/_NASASpaceApp/Blueprints/Player/BP_PlayerController.BP_PlayerController_C|GetWBPHUD _asbp_player_controller) (Variables|Default|GetText) (Variables|Default|GetDuration)))

(fn ConstructionScript)

(fn CanInteract
  (params (Caller :type Actor%20Object%20Reference))
  (return true))