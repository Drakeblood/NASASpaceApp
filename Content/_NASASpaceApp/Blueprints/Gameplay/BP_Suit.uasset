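; BP_Suit is an interactable suit that switches the interacting BP_HeroCharacter between two movement modes.
; Interact alternates the mode with a FlipFlop, held on the suit rather than per character, and sends it through ServerChangeMovementMode.
; Focus and Unfocus show and hide its Widget component, and CanInteract always allows interaction.
; A direct MulticastChangeMovementMode call is left unconnected.
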(event EventFocus
  (params (Caller :type Actor%20Object%20Reference))
  (Rendering|SetVisibility (Variables|Default|GetWidget) true false))

(event EventUnfocus
  (params (Caller :type BP%20Hero%20Character%20Object%20Reference))
  (Rendering|SetVisibility (Variables|Default|GetWidget) false false))

(event EventInteract
  (params (Caller :type Actor%20Object%20Reference))
  (bind _isa (Utilities|FlowControl|FlipFlop)
    (:A
      _)
    (:B
      _))
  (Default|ServerChangeMovementMode (.AsBP%20Hero%20Character (Utilities|Casting|CastToBP_HeroCharacter Caller)) (select _isa "NewEnumerator1" "NewEnumerator0")))

(fn ConstructionScript)

(fn CanInteract
  (params (Caller :type Actor%20Object%20Reference))
  (return true))