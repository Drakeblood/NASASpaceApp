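; BP_SolarPoint is a location marker that drives the scale of the BP_SolarPositionMeter actor by hero proximity.
; On authority, BeginPlay retries each tick until all players are valid, then caches the first player's hero and the meter.
; StartCheckingLocation enables tick, which maps the hero's 2D distance to a clamped uniform meter scale, growing to full size as the hero closes in.
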(event Custom|StartCheckingLocation
  (Actor|Tick|SetActorTickEnabled true))

(event EventTick
  (params (DeltaSeconds :type Float%20%28single-precision%29))
  (Transformation|SetActorScale3D (Variables|Default|GetSolarMeter) (Math|Conversions|ToVector(Float) (Math|Float|MapRangeClamped (Math|Vector|Distance2D(Vector) (Transformation|GetActorLocation (Variables|Default|GetHero)) (Transformation|GetActorLocation)) 1e+03 1e+02 0.0 1.0))))

(event EventBeginPlay
  (bind _nasagamemode (CallFunction|GetNASAGameMode))
  (Networking|SwitchHasAuthority
    (:Authority
      (if (Variables|/Game/_NASASpaceApp/Blueprints/System/GM_NASA.GM_NASA_C|GetbAllPlayersValid _nasagamemode) :!label _label
        (Variables|Default|SetHero (CallFunction|GetHerofromPlayerState (Utilities|Array|Get(acopy) (Variables|/Game/_NASASpaceApp/Blueprints/System/GM_NASA.GM_NASA_C|GetPlayers _nasagamemode))))
        (bind _returnvalue (Actor|GetActorOfClass "/Game/_NASASpaceApp/Blueprints/Gameplay/BP_SolarPositionMeter.BP_SolarPositionMeter_C"))
        (Variables|Default|SetSolarMeter _returnvalue)
        (else
          (Utilities|FlowControl|DelayUntilNextTick)
          (goto _label))))))

(fn ConstructionScript)