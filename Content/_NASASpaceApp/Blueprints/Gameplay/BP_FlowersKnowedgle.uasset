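; BP_FlowersKnowedgle is an interactable educational object that teaches the player about growing plants in space, such as NASA's Veggie system.
; Focus and Unfocus show and hide its Widget component, and CanInteract always allows interaction.
; Interact resolves the calling pawn's BP_PlayerController and shows a hard-coded timed dialogue text on its HUD widget.
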(event EventFocus
  (params (Caller :type Actor%20Object%20Reference))
  (Rendering|SetVisibility (Variables|Default|GetWidget) true false))

(event EventUnfocus
  (params (Caller :type BP%20Hero%20Character%20Object%20Reference))
  (Rendering|SetVisibility (Variables|Default|GetWidget) false false))

(event EventInteract
  (params (Caller :type Actor%20Object%20Reference))
  (bind _aspawn (Utilities|Casting|CastToPawn Caller))
  (bind _asbp_player_controller (Utilities|Casting|CastToBP_PlayerController (Pawn|GetController _aspawn)))
  (Default|ShowDialogue (Variables|/Game/_NASASpaceApp/Blueprints/Player/BP_PlayerController.BP_PlayerController_C|GetWBPHUD _asbp_player_controller) "In the history of space exploration there have been many succesful attempts to start and cultivate floral life in a space station's enviroment, both for practical and aesthetical reasons that could potentially benefit astronaut crew's physical and mental health. One of which is called the Vegetable Production System, also known as Veggie - a space garden that helps NASA understand behaviour of plants in a zero gravity enviroment, and also provide the mission's crew with freshly grown food." 1e+01))

(fn ConstructionScript)

(fn CanInteract
  (params (Caller :type Actor%20Object%20Reference))
  (return true))