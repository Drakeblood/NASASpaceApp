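; BP_Computer is an interactable computer actor that opens and closes a main computer screen UI for the player.
; Interact toggles a WBP_MainComputer widget on the viewport, creating it for player controller 0 or removing it if already open.
; Focus and Unfocus show or hide a Widget component, and ending overlap with the Sphere also closes the screen.
; CanInteract always returns true.
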(event OnComponentEndOverlap(Sphere)
  (params (OverlappedComponent :type Primitive%20Component%20Object%20Reference) (OtherActor :type Actor%20Object%20Reference) (OtherComp :type Primitive%20Component%20Object%20Reference) (OtherBodyIndex :type Integer))
  (bind _wbp (Variables|Default|GetWBP)
    (:then
      (Widget|RemovefromParent _wbp)
      (Variables|Default|SetWBP 0))
    (:else)))

(event EventBeginPlay)

(event Collision|EventActorBeginOverlap
  (params (OtherActor :type Actor%20Object%20Reference)))

(event EventTick
  (params (DeltaSeconds :type Float%20%28single-precision%29)))

(event EventFocus
  (params (Caller :type Actor%20Object%20Reference))
  (Rendering|SetVisibility (Variables|Default|GetWidget) true false))

(event EventUnfocus
  (params (Caller :type BP%20Hero%20Character%20Object%20Reference))
  (Rendering|SetVisibility (Variables|Default|GetWidget) false false))

(event EventInteract
  (params (Caller :type Actor%20Object%20Reference))
  (bind _wbp (Variables|Default|GetWBP)
    (:then
      (Widget|RemovefromParent _wbp)
      (Variables|Default|SetWBP 0))
    (:else
      (bind _returnvalue (UserInterface|CreateWidget "/Game/_NASASpaceApp/Blueprints/UI/WBP_MainComputer.WBP_MainComputer_C" (Game|GetPlayerController 0)))
      (bind _output_get (Variables|Default|SetWBP _returnvalue))
      (UserInterface|Viewport|AddtoViewport _output_get 0))))

(fn ConstructionScript)

(fn CanInteract
  (params (Caller :type Actor%20Object%20Reference))
  (return true))