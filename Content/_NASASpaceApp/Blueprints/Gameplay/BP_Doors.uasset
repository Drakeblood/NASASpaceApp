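; BP_Doors is a two-panel door that opens when something overlaps its sphere and closes when the overlap ends.
; BeginPlay converts local left and right destinations to world space, and overlaps play or reverse OpenDoorTimeline, whose rate the construction script derives from Duration.
; The timeline update lerps both panels toward those destinations, though the left starts from InitialRotation, which holds the actor's rotation rather than a location.
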(event OnComponentBeginOverlap(Sphere)
  (params (OverlappedComponent :type Primitive%20Component%20Object%20Reference) (OtherActor :type Actor%20Object%20Reference) (OtherComp :type Primitive%20Component%20Object%20Reference) (OtherBodyIndex :type Integer) (bFromSweep :type Boolean) (SweepResult :type Hit%20Result%20Structure%20%28by%20ref%29))
  (Variables|Default|SetPlaying true)
  (Audio|Components|Audio|Play (Variables|Default|GetOpenDoorTimeline)))

(event OnComponentEndOverlap(Sphere)
  (params (OverlappedComponent :type Primitive%20Component%20Object%20Reference) (OtherActor :type Actor%20Object%20Reference) (OtherComp :type Primitive%20Component%20Object%20Reference) (OtherBodyIndex :type Integer))
  (Variables|Default|SetPlaying true)
  (Utilities|String|Reverse (Variables|Default|GetOpenDoorTimeline)))

(event EventBeginPlay
  (Variables|Default|SetInitialRotation (Transformation|GetActorRotation))
  (Variables|Default|SetLeftDestinationWorldLocation (Math|Transform|TransformLocation (Transformation|GetActorTransform) (Variables|Default|GetLeftDestinationLocation)))
  (Variables|Default|SetRightDestinationWorldLocation (Math|Transform|TransformLocation (Transformation|GetActorTransform) (Variables|Default|GetRightDestinationLocation))))

(fn ConstructionScript
  (Components|Timeline|SetPlayRate (Variables|Default|GetOpenDoorTimeline) (/ 1.0 (Variables|Default|GetDuration))))