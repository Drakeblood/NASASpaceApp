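; BP_SuitKnowedgle is an interactable educational point that presents facts about NASA's Extravehicular Mobility Unit spacesuit.
; Interact casts the caller's controller to BP_PlayerController and shows a hardcoded text on its HUD as timed dialogue.
; Focus and Unfocus show and hide its Widget component, and CanInteract always allows interaction.
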(event EventFocus
  (params (Caller :type Actor%20Object%20Reference))
  (Rendering|SetVisibility (Variables|Default|GetWidget) true false))

(event EventUnfocus
  (params (Caller :type BP%20Hero%20Character%20Object%20Reference))
  (Rendering|SetVisibility (Variables|Default|GetWidget) false false))

(event EventInteract
  (params (Caller :type Actor%20Object%20Reference))
  (bind _aspawn (Utilities|Casting|CastToPawn Caller))
  (bind _asbp_player_controller (Utilities|Casting|CastToBP_PlayerController (Pawn|GetController _aspawn)))
  (Default|ShowDialogue (Variables|/Game/_NASASpaceApp/Blueprints/Player/BP_PlayerController.BP_PlayerController_C|GetWBPHUD _asbp_player_controller) "Extravehicular Mobility Unit (EMU) is a spacesuit specifically designed to perform tasks that require extravehicular activity (EVA). Designed to sustain life outside space stations, the suit provides enviromental protection, life support and communications. The development of the first NASA's EMU started in 1974 and it was first flown in 1981, and it had gone over partial redesigns over the 40 years of usage. The outer parts of the EMU contain two major components - the Pressure Garment System (PGS), responsible for maintaining appropriate pressure around human body in the vacuum of space, while also allowing for proper mobility for operations, and the Primary Life Support System (PLSS), a device resembling a backpack with functions required to keep the human body alive during extravehicular activity, like providing oxygen, maintaining body temperature, and also removing carbon dioxide and humidity from the suit." 15.0))

(fn ConstructionScript)

(fn CanInteract
  (params (Caller :type Actor%20Object%20Reference))
  (return true))