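; GM_NASA, apparently a game mode, places two players at their spawn points once both have registered.
; AddValidPlayer appends to the Players array and fires AllPlayersValid when the new entry lands at index 1, the second slot.
; That event finds the Player 1 and Player 2 spawn point actors and moves each player's pawn to the matching location without sweep or teleport.
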(event Custom|AllPlayersValid
  (bind _returnvalue (Actor|GetActorOfClass "/Game/_NASASpaceApp/Blueprints/Gameplay/BP_Player1SpawnPoint.BP_Player1SpawnPoint_C"))
  (Transformation|SetActorLocation (PlayerState|GetPawn (Utilities|Array|Get(acopy) (Variables|Default|GetPlayers))) (Transformation|GetActorLocation _returnvalue) false false)
  (bind _returnvalue_2 (Actor|GetActorOfClass "/Game/_NASASpaceApp/Blueprints/Gameplay/BP_Player2SpawnPoint.BP_Player2SpawnPoint_C"))
  (Transformation|SetActorLocation (PlayerState|GetPawn (Utilities|Array|Get(acopy) (Variables|Default|GetPlayers) 1)) (Transformation|GetActorLocation _returnvalue_2) false false))

(fn ConstructionScript)

(fn AddValidPlayer
  (params (NewItem :type BP%20Player%20State%20Object%20Reference%20%28by%20ref%29))
  (bind _returnvalue (Utilities|Array|Add (Variables|Default|GetPlayers) NewItem))
  (if (== _returnvalue 1)
    (CallFunction|AllPlayersValid)))