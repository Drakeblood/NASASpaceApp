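; Blueprint function library for the NASA Space App project that provides typed shortcuts to core framework objects.
; It returns the game instance as BP_GameInstance and the game mode as GM_NASA.
; It also resolves a player state's pawn to BP_HeroCharacter.
; Each helper is a single getter followed by a cast.
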(fn GetNASAGameInstance
  (return (.AsBP%20Game%20Instance (Utilities|Casting|CastToBP_GameInstance (Game|GetGameInstance)))))

(fn GetNASAGameMode
  (params (__WorldContext :type Object%20Object%20Reference))
  (return (.AsGM%20NASA (Utilities|Casting|CastToGM_NASA (Game|GetGameMode)))))

(fn GetHerofromPlayerState
  (params (PlayerState :type BP%20Player%20State%20Object%20Reference))
  (return (.AsBP%20Hero%20Character (Utilities|Casting|CastToBP_HeroCharacter (PlayerState|GetPawn PlayerState)))))